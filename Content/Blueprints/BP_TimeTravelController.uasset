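; BP_TimeTravelController manages the visual effects for the time travel recall ability, using the owner's capsule component and mesh.
; Each Tick polls IsRecallActive, attaching a Niagara haze to the capsule when recall starts and destroying it when recall ends.
; A validity check on the stored haze component prevents duplicate spawns.
; An afterimage effect on the mesh is present but never runs and is noted as not working.
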(event EventTick
  (params (DeltaSeconds :type Float%20%28single-precision%29))
  ;[0.4 0.8 1] Haze Spawn and Despawn
  (if (and (Variables|Default|GetIsRecallActive) (not (Utilities|IsValid (stale _returnvalue))))
    (bind _returnvalue (Niagara|SpawnSystemAttached "/Game/ParticleEffects/Haze/N_HazeSystem.N_HazeSystem" (Variables|Default|GetCapsuleComponent) "None" "0, 0, 0" "0, 0, 0" "KeepRelativeOffset" false))
    (elif (and (not (Variables|Default|GetIsRecallActive)) (Utilities|IsValid _returnvalue))
      (Components|DestroyComponent _returnvalue))))

(fn ConstructionScript)